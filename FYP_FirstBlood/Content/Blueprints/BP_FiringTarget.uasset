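; BP_FiringTarget is a shooting target that tips over when hit via Interact and can optionally stand back up.
; A timeline rolls RotationRoot and turns Cube1 red, then TargetHitAudio plays a temporary sound, guarded by the Shot flag.
; If Reactivate is set, a delayed second timeline rotates it back, applies BasicShapeMaterial and clears Shot.
; The construction script gives non-enemy targets the GoodTarget material on both cubes.
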(event Custom|Reactivate
  (bind _newtrack_0 (Timeline|Timeline_0 PlayFromStart)
    (:Update
      (Transformation|SetRelativeRotation (Variables|Default|GetRotationRoot) (Math|Rotator|MakeRotator _newtrack_0 0.0 0.0) false false)
      (Rendering|Material|SetMaterial (Variables|Default|GetCube1) 0 "/Engine/BasicShapes/BasicShapeMaterial.BasicShapeMaterial"))
    (:Finished
      (Variables|Default|SetShot? false))))

(event EventInteract
  (bind _newtrack_0 (Timeline|Timeline_1 Play)
    (:Update
      (Transformation|SetRelativeRotation (Variables|Default|GetRotationRoot) (Math|Rotator|MakeRotator _newtrack_0 0.0 0.0) false false)
      (Rendering|Material|SetMaterial (Variables|Default|GetCube1) 0 "/Game/Materials/RED.RED"))
    (:Finished
      (|TargetHitAudio)
      (if (Variables|Default|GetReactivate?)
        (Utilities|FlowControl|Delay 3.0)
        (CallFunction|Reactivate)
        (Timeline|Timeline_1 SetNewTime)))))

(fn ConstructionScript
  (if (not (Variables|Default|GetEnemy?))
    (Rendering|Material|SetMaterial (Variables|Default|GetCube1) 0 "/Game/Materials/GoodTarget.GoodTarget")))