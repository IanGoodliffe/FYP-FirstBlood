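; Leaderboard actor that shows the top five course times on text render components and persists them in a BP_SaveGame slot.
; On BeginPlay it loads the saved times, creating placeholder defaults if no save exists.
; Sorting orders times ascending by repeatedly extracting the minimum, drops the sixth entry and refreshes the board.
; DisplayTimes formats seconds as minutes:seconds, highlights the entry matching the player HUD's result, then saves.
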(event Custom|Sorting
  (bind _storedtimes (Variables|Default|GetStoredTimes))
  (bind _sortedtimes (Variables|Default|GetSortedTimes))
  (bind _storedtimes_2 (Variables|Default|GetStoredTimes))
  (bind (_indexofminvalue _minvalue) (Math|Integer|MinOfIntArray _storedtimes))
  ;[1 1 1] SortArrays
  (while (> (Utilities|Array|Length (Variables|Default|GetStoredTimes)) 0)
    (Utilities|Array|Add (Variables|Default|GetSortedTimes) _minvalue)
    (Utilities|Array|RemoveIndex _storedtimes _indexofminvalue))
  (for _array_element _sortedtimes
    (Utilities|Array|Add _storedtimes_2 _array_element))
  (Utilities|Array|Clear _sortedtimes)
  (Utilities|Array|RemoveIndex _storedtimes_2 5)
  (CallFunction|DisplayTimes))

(event Custom|DisplayTimes
  (bind _returnvalue (Game|GetPlayerCharacter 0))
  (bind _times (Variables|Default|GetTimes))
  (bind _timerenderers (Variables|Default|GetTimeRenderers))
  (bind _asbp_player (Utilities|Casting|CastToBP_Player _returnvalue))
  (bind _playerhud (Variables|/Game/Blueprints/BP_Player.BP_Player_C|GetPlayerHud _asbp_player))
  (bind _timeresult (Variables|/Game/UI_Assets/BP_HUD.BP_HUD_C|GetTimeResult _playerhud))
  (bind _returnvalue_2 (Utilities|Array|FindItem _times _timeresult))
  (bind _output (Utilities|Array|Get(acopy) _timerenderers _returnvalue_2))
  ;[1 1 1] DisplayTimes
  (Utilities|Array|Clear (Variables|Default|GetTimeRenderers))
  (CallFunction|ResetText)
  (for _array_element (Variables|Default|GetStoredTimes)
    (bind _output_get (Variables|Default|SetCurrentTime _array_element))
    (if (>= _output_get 60) :!label _label
      (Variables|Default|SetTimeInMins (+ (Variables|Default|GetTimeInMins) 1))
      (Variables|Default|SetCurrentTime (- _output_get 60))
      (goto _label)
      (else
        (Variables|Default|SetTimeInSeconds _output_get)
        (Utilities|Array|Add (Variables|Default|GetTimes) (Utilities|Text|FormatText "{Mins}:{Secs}" (Utilities|Text|ToText(Integer) (Variables|Default|GetTimeInMins)) (Utilities|Text|ToText(Integer) (Variables|Default|GetTimeInSeconds) false true 2)))
        (Variables|Default|SetTimeInMins 0)
        (Variables|Default|SetTimeInSeconds 0))))
  (for (_array_element_2 _array_index) (Variables|Default|GetTimes)
    (Rendering|Components|TextRender|SetText (Utilities|Array|Get(acopy) (Variables|Default|GetTimeRenderers) _array_index) _array_element_2))
  (Utilities|IsValid _playerhud
    (:Is%20Valid
      (for _array_element_3 _timerenderers
        (Rendering|Components|TextRender|SetTextRenderColor _array_element_3 (Math|Color|MakeColor 0 0 0)))
      (Utilities|IsValid _output
        (:Is%20Valid
          (Rendering|Components|TextRender|SetTextRenderColor _output (Math|Color|MakeColor 0 60 255))
          (Utilities|Array|Clear (Variables|Default|GetTimes))
          (CallFunction|SaveData))))
    (:Is%20Not%20Valid
      (Utilities|Array|Clear _times))))

(event Custom|ResetText
  (bind _timerenderers (Variables|Default|GetTimeRenderers))
  ;[1 1 1] SetTextRenderers
  (Utilities|Array|Add _timerenderers (Variables|Default|GetTopTime))
  (Utilities|Array|Add _timerenderers (Variables|Default|GetTopTime1))
  (Utilities|Array|Add _timerenderers (Variables|Default|GetTopTime2))
  (Utilities|Array|Add _timerenderers (Variables|Default|GetTopTime3))
  (Utilities|Array|Add _timerenderers (Variables|Default|GetTopTime4)))

(event EventBeginPlay
  (bind _timerenderers (Variables|Default|GetTimeRenderers))
  ;[1 1 1] SetTextRenderers
  (CallFunction|DoesSaveExist?)
  (bind _bpsave (CallFunction|LoadData))
  (Variables|Default|SetStoredTimes (Variables|/Game/Blueprints/BP_SaveGame.BP_SaveGame_C|GetSavedTimes _bpsave))
  (CallFunction|DisplayTimes)
  (Utilities|Array|Add _timerenderers (Variables|Default|GetTopTime))
  (Utilities|Array|Add _timerenderers (Variables|Default|GetTopTime1))
  (Utilities|Array|Add _timerenderers (Variables|Default|GetTopTime2))
  (Utilities|Array|Add _timerenderers (Variables|Default|GetTopTime3))
  (Utilities|Array|Add _timerenderers (Variables|Default|GetTopTime4)))

(fn ConstructionScript)

(fn DoesSaveExist?
  (bind _returnvalue (SaveGame|DoesSaveGameExist "Default"))
  (if _returnvalue
    (bind _returnvalue_2 (SaveGame|LoadGamefromSlot "Default"))
    (return _returnvalue_2)
    (else
      (bind _returnvalue_3 (SaveGame|CreateSaveGameObject "/Game/Blueprints/BP_SaveGame.BP_SaveGame_C"))
      (Variables|/Game/Blueprints/BP_SaveGame.BP_SaveGame_C|SetSavedTimes _returnvalue_3 (Utilities|Array|MakeArray 100 200 300 400 500))
      (SaveGame|SaveGametoSlot _returnvalue_3 "Default")
      (return _returnvalue_3))))

(fn SaveData
  (bind _savegame (CallFunction|DoesSaveExist?))
  (bind _asbp_save_game (Utilities|Casting|CastToBP_SaveGame _savegame))
  (Variables|/Game/Blueprints/BP_SaveGame.BP_SaveGame_C|SetSavedTimes _asbp_save_game (Variables|Default|GetStoredTimes))
  (bind _returnvalue (SaveGame|SaveGametoSlot _savegame "Default"))
  (return _returnvalue))

(fn LoadData
  (bind _returnvalue (SaveGame|DoesSaveGameExist "Default"))
  (if _returnvalue
    (bind _returnvalue_2 (SaveGame|LoadGamefromSlot "Default"))
    (bind _asbp_save_game (Utilities|Casting|CastToBP_SaveGame _returnvalue_2))
    (return _asbp_save_game)))