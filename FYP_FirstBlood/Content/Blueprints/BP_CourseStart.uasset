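; BP_CourseStart is the start trigger of a timed target-shooting course.
; When the player enters TimerHitbox, it moves the civilian to a fixed spot, shows the HUD timer and resets every target.
; After a short delay placed inside the target loop, it enables collision on its Blocking component to close the entrance.
; It also disables blocking on the BP_CourseEnd found at BeginPlay, opening that end.
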(event OnComponentBeginOverlap(TimerHitbox)
  (params (OverlappedComponent :type Primitive%20Component%20Object%20Reference) (OtherActor :type Actor%20Object%20Reference) (OtherComp :type Primitive%20Component%20Object%20Reference) (OtherBodyIndex :type Integer) (bFromSweep :type Boolean) (SweepResult :type Hit%20Result%20Structure%20%28by%20ref%29))
  (bind (_asbp_player _bsuccess) (Utilities|Casting|CastToBP_Player OtherActor))
  (if _bsuccess
    (Transformation|SetWorldLocation (Variables|/Game/Blueprints/BP_FiringTarget.BP_FiringTarget_C|GetDefaultSceneRoot (Variables|Default|GetCivillian)) "2472.103516,-488.000000, 0" false false)
    (Default|TimerAppear (Variables|/Game/Blueprints/BP_Player.BP_Player_C|GetPlayerHud _asbp_player))
    (for _array_element (Variables|Default|GetTargets)
      (Variables|/Game/Blueprints/BP_FiringTarget.BP_FiringTarget_C|SetShot? _array_element false)
      (Default|CourseRestart _array_element)
      (Utilities|FlowControl|Delay 0.25)
      (CallFunction|BlockEntrance)
      (Collision|SetCollisionEnabled (Variables|/Game/Blueprints/BP_CourseEnd.BP_CourseEnd_C|GetBlocking (Variables|Default|GetCourseEndRef)) "NoCollision"))))

(event Custom|BlockEntrance
  (Collision|SetCollisionEnabled (Variables|Default|GetBlocking) "QueryOnly"))

(event EventBeginPlay
  (Collision|SetCollisionEnabled (Variables|Default|GetBlocking) "NoCollision")
  (bind _returnvalue (Actor|GetActorOfClass "/Game/Blueprints/BP_CourseEnd.BP_CourseEnd_C"))
  (Variables|Default|SetCourseEndRef _returnvalue))

(event Collision|EventActorBeginOverlap
  (params (OtherActor :type Actor%20Object%20Reference)))

(event EventTick
  (params (DeltaSeconds :type Float%20%28single-precision%29)))

(fn ConstructionScript)