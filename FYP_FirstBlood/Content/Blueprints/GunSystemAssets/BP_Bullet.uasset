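; BP_Bullet is a physics-driven bullet projectile with a particle trail for the gun system.
; Its Init event randomly destroys one in four bullets immediately.
; The rest tint the BulletTrail particles, launch BulletBody forward with a mass-independent force and expire after a short lifespan.
; It contains no hit, overlap or damage logic.
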(event Custom|Init
  (if (== (Math|Random|RandomIntegerinRange 1 4) 4)
    (Actor|DestroyActor)
    (else
      (Niagara|SetNiagaraVariable(LinearColor) (Variables|Default|GetBulletTrail) "ParticleColor" (Math|Color|MakeColor 0.25 0.15 0.15))
      (Physics|AddForce (Variables|Default|GetBulletBody) (* (Math|Vector|GetForwardVector (Transformation|GetWorldRotation (Variables|Default|GetBulletBody))) 1e+06) "None" true)
      (Actor|SetLifeSpan 3.0))))

(event Collision|EventActorBeginOverlap
  (params (OtherActor :type Actor%20Object%20Reference)))

(event EventTick
  (params (DeltaSeconds :type Float%20%28single-precision%29)))

(fn ConstructionScript)