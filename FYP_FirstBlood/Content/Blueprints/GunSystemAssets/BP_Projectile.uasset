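; BP_Projectile is a thrown projectile for the gun system, with grenade as the only type implemented in its Init switch.
; Init swaps in the grenade mesh, launches it forward with a physics force, then triggers detonation after a short fuse.
; Detonation hides the mesh, plays sound, Niagara and a light flash, while a timeline scales the hitbox sphere before cleanup.
; Actors overlapping the sphere receive an InteractMessage call.
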(event OnComponentBeginOverlap(Sphere)
  (params (OverlappedComponent :type Primitive%20Component%20Object%20Reference) (OtherActor :type Actor%20Object%20Reference) (OtherComp :type Primitive%20Component%20Object%20Reference) (OtherBodyIndex :type Integer) (bFromSweep :type Boolean) (SweepResult :type Hit%20Result%20Structure%20%28by%20ref%29))
  (Class|BulletInteract|Interact(Message) (.hitactor SweepResult) "None" "0, 0, 0"))

(event Custom|Init
  (params (NewParam :type ProjectileTypes%20Enum :default "NewEnumerator0"))
  (switch Utilities|FlowControl|Switch|SwitchonProjectileTypes NewParam
    (:NewEnumerator0
      (|Grenade) ; enters at execute2
    )))

(fn ConstructionScript)