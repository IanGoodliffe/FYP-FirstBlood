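; BP_FiringTarget is a target that rotates when interacted with, then resets itself after a short pause.
; Interact plays a timeline that rolls RotationRoot and turns Cube1 red.
; When that finishes, a delay leads to Reactivate, whose own timeline drives the roll and restores the basic material.
; The first timeline's time is then reset for the next interaction.
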(event Custom|Reactivate
  (bind _newtrack_0 (Timeline|Timeline_0 PlayFromStart)
    (:Update
      (Transformation|SetRelativeRotation (Variables|Default|GetRotationRoot) (Math|Rotator|MakeRotator _newtrack_0 0.0 0.0) false false)
      (Rendering|Material|SetMaterial (Variables|Default|GetCube1) 0 "/Engine/BasicShapes/BasicShapeMaterial.BasicShapeMaterial"))))

(event EventInteract
  (bind _newtrack_0 (Timeline|Timeline_1 Play)
    (:Update
      (Transformation|SetRelativeRotation (Variables|Default|GetRotationRoot) (Math|Rotator|MakeRotator _newtrack_0 0.0 0.0) false false)
      (Rendering|Material|SetMaterial (Variables|Default|GetCube1) 0 "/Game/RED.RED"))
    (:Finished
      (Utilities|FlowControl|Delay 3.0)
      (CallFunction|Reactivate)
      (Timeline|Timeline_1 SetNewTime))))

(fn ConstructionScript)