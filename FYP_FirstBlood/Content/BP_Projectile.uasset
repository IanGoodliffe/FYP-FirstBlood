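; Projectile actor that launches forward, then turns into an expanding overlap sphere, similar to a timed blast.
; Init applies a large physics force along the static mesh's forward vector, then hides the mesh after a short delay.
; A timeline then drives the sphere's world scale, and a brief life span removes the actor when it finishes.
; Sphere overlaps only print the other actor's name; no damage is applied.
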(event OnComponentBeginOverlap(Sphere)
  (params (OverlappedComponent :type Primitive%20Component%20Object%20Reference) (OtherActor :type Actor%20Object%20Reference) (OtherComp :type Primitive%20Component%20Object%20Reference) (OtherBodyIndex :type Integer) (bFromSweep :type Boolean) (SweepResult :type Hit%20Result%20Structure%20%28by%20ref%29))
  (Development|PrintString (Utilities|GetDisplayName OtherActor)))

(event Custom|Init
  (Physics|AddForce (Variables|Default|GetStaticMesh) (* (Math|Vector|GetForwardVector (Transformation|GetWorldRotation (Variables|Default|GetStaticMesh))) 2e+05) "None" false)
  (Utilities|FlowControl|Delay 1.0)
  (Rendering|SetVisibility (Variables|Default|GetStaticMesh) false false)
  (bind _newtrack_0 (Timeline|Timeline_0 Play)
    (:Update
      (Transformation|SetWorldScale3D (Variables|Default|GetSphere) _newtrack_0))
    (:Finished
      (Actor|SetLifeSpan 0.3))))

(fn ConstructionScript)